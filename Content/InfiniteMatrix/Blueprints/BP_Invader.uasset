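; BP_Invader is an enemy actor that reacts when its static mesh overlaps the player or a missile.
; Hitting the player applies the player's collision damage through ChangeHealth, then either shows the restart screen on death or shakes the camera and destroys the invader's mesh component.
; Hitting a missile destroys both actors and increments the player's score and score display, handled inline while ProcessInvaderHit remains an empty stub.
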(event OnComponentBeginOverlap(StaticMesh)
  (params (OverlappedComponent :type Primitive%20Component%20Object%20Reference) (OtherActor :type Actor%20Object%20Reference) (OtherComp :type Primitive%20Component%20Object%20Reference) (OtherBodyIndex :type Integer) (bFromSweep :type Boolean) (SweepResult :type Hit%20Result%20Structure%20%28by%20ref%29))
  (bind _returnvalue (Game|Player|GetPlayerPawn 0))
  (bind _asbp_player (Utilities|Casting|CastToBP_Player _returnvalue))
  (Utilities|FlowControl|Sequence
    (:then_0
      (bind _asbp_player_2 (Utilities|Casting|CastToBP_Player OtherActor))
      (CallFunction|ProcessPlayerHit _asbp_player_2))
    (:then_1
      (bind _asbp_missile (Utilities|Casting|CastToBP_Missile OtherActor))
      (Actor|DestroyActor _asbp_missile)
      (bind _output_get (Variables|/Game/InfiniteMatrix/Blueprints/BP_Player.BP_Player_C|SetScore _asbp_player (+ (Variables|/Game/InfiniteMatrix/Blueprints/BP_Player.BP_Player_C|GetScore _asbp_player) 1)))
      (Default|UpdateScoreDisplay (Variables|/Game/InfiniteMatrix/Blueprints/BP_Player.BP_Player_C|GetScoreDisplayReference _asbp_player) _output_get)
      (Actor|DestroyActor))))

(event EventBeginPlay)

(event Collision|EventActorBeginOverlap
  (params (OtherActor :type Actor%20Object%20Reference)))

(event EventTick
  (params (DeltaSeconds :type Float%20%28single-precision%29)))

(fn ConstructionScript)

(fn ProcessPlayerHit
  (params (Actor%20Ref :type BP%20Player%20Object%20Reference))
  (bind _health (Default|ChangeHealth Actor%20Ref (Variables|/Game/InfiniteMatrix/Blueprints/BP_Player.BP_Player_C|GetCollisionDamage Actor%20Ref)))
  (if (<= _health 0.0)
    (Variables|/Game/InfiniteMatrix/Blueprints/BP_Player.BP_Player_C|SetIsDead Actor%20Ref true)
    (Default|DisplayRestart Actor%20Ref)
    (else
      (Camera|PlayWorldCameraShake "/Game/InfiniteMatrix/Blueprints/BP_CameraShake.BP_CameraShake_C" (Transformation|GetActorLocation (Game|Player|GetPlayerPawn 0)) 0.0 5e+02)
      (Components|DestroyComponent (Variables|Default|GetStaticMesh)))))

(fn ProcessInvaderHit)