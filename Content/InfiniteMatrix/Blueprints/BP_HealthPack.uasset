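; BP_HealthPack is a spinning health pickup actor that heals the player on overlap.
; When a BP_Player overlaps it, the pack calls ChangeHealth to add health only if the player is below full, then destroys itself either way.
; Tick yaws the static mesh by DeltaSeconds times RotateSpeed for a frame-rate independent spin.
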(event EventBeginPlay)

(event Collision|EventActorBeginOverlap
  (params (OtherActor :type Actor%20Object%20Reference))
  (bind _asbp_player (Utilities|Casting|CastToBP_Player OtherActor))
  (if (< (Variables|/Game/InfiniteMatrix/Blueprints/BP_Player.BP_Player_C|GetHealth _asbp_player) 1e+02)
    (Default|ChangeHealth _asbp_player 2e+01))
  (Actor|DestroyActor))

(event EventTick
  (params (DeltaSeconds :type Float%20%28single-precision%29))
  (Transformation|AddLocalRotation (Variables|Default|GetStaticMesh) (Math|Rotator|MakeRotator 0.0 0.0 (* DeltaSeconds (Variables|Default|GetRotateSpeed))) false false))

(fn ConstructionScript)